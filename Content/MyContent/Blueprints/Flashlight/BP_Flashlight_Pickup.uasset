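; BP_Flashlight_Pickup is a collectible that gives the player the flashlight.
; On BeginPlay it casts player 0's character to BP_FirstPersonCharacter and caches the reference.
; When that character overlaps the capsule, it sets the character's HasFlashlight flag, plays a collect sound at the pickup's location and destroys itself.
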(event OnComponentBeginOverlap(Capsule)
  (params (OverlappedComponent :type Primitive%20Component%20Object%20Reference) (OtherActor :type Actor%20Object%20Reference) (OtherComp :type Primitive%20Component%20Object%20Reference) (OtherBodyIndex :type Integer) (bFromSweep :type Boolean) (SweepResult :type Hit%20Result%20Structure%20%28by%20ref%29))
  (bind _bp_first_person_character (Variables|Default|GetBP_First_Person_Character))
  ;[0.15 0.15 0.15 0.5] Collect Flashlight
  (if (== OtherActor _bp_first_person_character)
    (Variables|/Game/StarterContent/FirstPerson/Blueprints/BP_FirstPersonCharacter.BP_FirstPersonCharacter_C|SethasFlashlight _bp_first_person_character true)
    (Audio|PlaySoundatLocation "/Game/MyContent/Audio/MP3_Key_Collect.MP3_Key_Collect" (Transformation|GetActorLocation) "0, 0, 0" 1.0 1.0 0.0 0 0 0 0)
    (Actor|DestroyActor)))

(event EventBeginPlay
  ;[0.15 0.15 0.15 0.5] Flashligh Setup
  (bind _asbp_first_person_character (Utilities|Casting|CastToBP_FirstPersonCharacter (Game|GetPlayerCharacter 0)))
  (Variables|Default|SetBP_First_Person_Character _asbp_first_person_character))

(event Collision|EventActorBeginOverlap
  (params (OtherActor :type Actor%20Object%20Reference)))

(event EventTick
  (params (DeltaSeconds :type Float%20%28single-precision%29)))

(fn ConstructionScript)