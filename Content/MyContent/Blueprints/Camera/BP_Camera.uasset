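; A sweeping security camera that catches the player and restarts the stealth level.
; From BeginPlay, a self-repeating MoveCamera event uses FlipFlop and MoveComponentTo to swing the eyeball mesh between start and end rotations, with a delay between moves.
; Every Tick, a debug-drawn Pawn line trace runs forward from the trace mesh.
; Hitting the cached first-person character prints a message, disables input, then reopens StealthLevel after a short delay.
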(event Custom|Detect
  (bind _sm_linetrace (Variables|Default|GetSM_LineTrace))
  (bind _returnvalue (Transformation|GetWorldLocation _sm_linetrace))
  ;[0.15 0.15 0.15 0.5] Detection
  (bind _outhit (Collision|LineTraceForObjects _returnvalue (+ _returnvalue (* (Math|Vector|GetForwardVector (Transformation|GetWorldRotation _sm_linetrace)) (Variables|Default|GetDetectDistance))) (Utilities|Array|MakeArray "ObjectTypeQuery3") false 0 "ForOneFrame"))
  (if (== (.HitActor (Collision|BreakHitResult _outhit)) (Variables|Default|GetBP_First_Person_Character))
    (Development|PrintString "PERCIEVED")
    ;[0.15 0.15 0.15 0.5] Disable Input and Reset Level
    (Input|DisableInput (Variables|Default|GetBP_First_Person_Character) (Game|GetPlayerController 0))
    (Utilities|FlowControl|Delay 1.0)
    (Game|OpenLevel(byName) "StealthLevel")))

(event Custom|Move%20Camera
  ;[0.15 0.15 0.15 0.5] Camera Movement
  (Utilities|FlowControl|FlipFlop
    (:A
      (Variables|Default|SetCurrentRotation (Variables|Default|GetEndRotation)))
    (:B
      (Variables|Default|SetCurrentRotation (Variables|Default|GetSartRotation))))
  (Components|MoveComponentTo (Variables|Default|GetSM_EyeballCam) "0, 0, 0" (Math|Rotator|MakeRotator (.x (Variables|Default|GetCurrentRotation)) (.y (Variables|Default|GetCurrentRotation)) (.z (Variables|Default|GetCurrentRotation))) false false (Variables|Default|GetSpeed) false)
  (Utilities|FlowControl|Delay (Variables|Default|GetDelay))
  (CallFunction|MoveCamera))

(event EventBeginPlay
  ;[0.15 0.15 0.15 0.5] Reference
  (CallFunction|MoveCamera)
  (bind _asbp_first_person_character (Utilities|Casting|CastToBP_FirstPersonCharacter (Game|GetPlayerCharacter 0)))
  (Variables|Default|SetBP_First_Person_Character _asbp_first_person_character))

(event Collision|EventActorBeginOverlap
  (params (OtherActor :type Actor%20Object%20Reference)))

(event EventTick
  (params (DeltaSeconds :type Float%20%28single-precision%29))
  (CallFunction|Detect))

(fn ConstructionScript)