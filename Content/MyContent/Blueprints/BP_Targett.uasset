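; BP_Targett is a moving target actor that oscillates along a line and is destroyed after enough hits.
; A looping timer negates Direction every MovementDur, while Tick offsets the actor along the normalized Direction by Speed per frame, without delta-time scaling or sweep.
; Its Hit event decrements HP, spawns a Niagara effect and sound at the hit location, and destroys the actor once HP reaches zero.
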(event Custom|Evet_FlipDirection
  (Variables|Default|SetDirection (* (Variables|Default|GetDirection) -1.0)))

(event EventBeginPlay
  (Utilities|Time|SetTimerbyEvent (delegate Custom|Evet_FlipDirection) (Variables|Default|GetMovementDur) true))

(event EventTick
  (params (DeltaSeconds :type Float%20%28single-precision%29))
  (Transformation|AddActorWorldOffset (* (Math|Vector|Normalize (Variables|Default|GetDirection)) (Variables|Default|GetSpeed))))

(event Collision|EventHit
  (params (MyComp :type Primitive%20Component%20Object%20Reference) (Other :type Actor%20Object%20Reference) (OtherComp :type Primitive%20Component%20Object%20Reference) (bSelfMoved :type Boolean) (HitLocation :type Vector :default "0, 0, 0") (HitNormal :type Vector :default "0, 0, 0") (NormalImpulse :type Vector :default "0, 0, 0") (Hit :type Hit%20Result%20Structure%20%28by%20ref%29))
  (Variables|Default|SetHP (- (Variables|Default|GetHP) 1))
  (if (<= (Variables|Default|GetHP) 0)
    (Niagara|SpawnSystematLocation "/Game/MyContent/FX/PE_Target_Hit.PE_Target_Hit" HitLocation)
    (Audio|SpawnSoundatLocation 0 HitLocation "0, 0, 0" 1.0 1.0 0.0 0 0)
    (Actor|DestroyActor)
    (else
      (Niagara|SpawnSystematLocation "/Game/MyContent/FX/PE_Target_Hit.PE_Target_Hit" HitLocation)
      (Audio|SpawnSoundatLocation 0 HitLocation "0, 0, 0" 1.0 1.0 0.0 0 0))))

(fn ConstructionScript)