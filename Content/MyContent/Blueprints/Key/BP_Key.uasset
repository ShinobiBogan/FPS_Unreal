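; BP_Key is a collectible key that stays hidden and non-collidable until no BP_Targett actors remain in the level.
; Tick polls the target count each frame to set visibility and collision, with a DoOnce spawning an effect and sound when the key appears.
; Once revealed, overlap by the cached first-person character sets its HasKey flag, plays a collect sound and destroys the key.
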(event OnComponentBeginOverlap(Collision)
  (params (OverlappedComponent :type Primitive%20Component%20Object%20Reference) (OtherActor :type Actor%20Object%20Reference) (OtherComp :type Primitive%20Component%20Object%20Reference) (OtherBodyIndex :type Integer) (bFromSweep :type Boolean) (SweepResult :type Hit%20Result%20Structure%20%28by%20ref%29))
  ;[0.15 0.15 0.15 0.5] Collecting the key
  (if (and (== OtherActor (Variables|Default|GetBP_FirstPersonCharacter)) (Variables|Default|GetAllTargetsDetroyed))
    (Variables|/Game/StarterContent/FirstPerson/Blueprints/BP_FirstPersonCharacter.BP_FirstPersonCharacter_C|SetHasKey (Variables|Default|GetBP_FirstPersonCharacter) true)
    (Audio|PlaySoundatLocation "/Game/MyContent/Audio/MP3_Key_Collect.MP3_Key_Collect" (Transformation|GetActorLocation) "0, 0, 0" 1.0 1.0 0.0 0 0 0 0)
    (Actor|DestroyActor)))

(event EventBeginPlay
  ;[0.15 0.15 0.15 0.5] Targets destroyed = Key Appear Functions
  (bind _asbp_first_person_character (Utilities|Casting|CastToBP_FirstPersonCharacter (Game|GetPlayerCharacter 0)))
  (Variables|Default|SetBP_FirstPersonCharacter _asbp_first_person_character))

(event Collision|EventActorBeginOverlap
  (params (OtherActor :type Actor%20Object%20Reference)))

(event EventTick
  (params (DeltaSeconds :type Float%20%28single-precision%29))
  (bind _sm_key (Variables|Default|GetSM_Key))
  (bind _returnvalue (Transformation|GetWorldLocation _sm_key))
  ;[0.15 0.15 0.15 0.5] Targets destroyed = Key Appear Functions
  (bind _outactors (Actor|GetAllActorsOfClass "/Game/MyContent/Blueprints/BP_Targett.BP_Targett_C"))
  (bind _returnvalue_2 (Utilities|Array|Add _outactors 0))
  (bind _output_get (Variables|Default|SetAllTargetsDetroyed (<= _returnvalue_2 0)))
  (Rendering|SetVisibility (Variables|Default|GetSM_Key) _output_get true)
  (Collision|SetActorEnableCollision _output_get)
  (if (Variables|Default|GetAllTargetsDetroyed)
    (Utilities|FlowControl|DoOnce false
      (:Completed
        (Niagara|SpawnSystematLocation "/Game/MyContent/FX/PE_Target_Hit.PE_Target_Hit" _returnvalue "0, 0, 0" "1.000000,1.000000,1.000000" true true "AutoRelease")
        (Audio|SpawnSoundatLocation "/Game/MyContent/Audio/MP3_Key_Appear.MP3_Key_Appear" _returnvalue "0, 0, 0" 1.0 1.0 0.0 0 0)))))

(fn ConstructionScript)