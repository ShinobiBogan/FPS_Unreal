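; BP_Door is a key-locked door that swings open for the first-person player and shows access through a coloured light.
; BeginPlay caches the player character and gives the light mesh a dynamic material instance.
; Entering the collision brightens the light, turning it green and playing the Timeline-driven rotation with a key, or red without one.
; Leaving restores the default colour and reverses the Timeline, but never resets the Intensity parameter.
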(event OnComponentBeginOverlap(DoorCollision)
  (params (OverlappedComponent :type Primitive%20Component%20Object%20Reference) (OtherActor :type Actor%20Object%20Reference) (OtherComp :type Primitive%20Component%20Object%20Reference) (OtherBodyIndex :type Integer) (bFromSweep :type Boolean) (SweepResult :type Hit%20Result%20Structure%20%28by%20ref%29))
  (bind _dynamicmaterial (Variables|Default|GetDynamicMaterial))
  ;[0.15 0.15 0.15 0.5] Overlap Light Change
  (if (== OtherActor (Variables|Default|GetBP_FirstPersonCharacter))
    (Rendering|Material|SetScalarParameterValue _dynamicmaterial "Intensity" 1e+02 :!class /Script/Engine.MaterialInstanceDynamic)
    (if (Variables|/Game/StarterContent/FirstPerson/Blueprints/BP_FirstPersonCharacter.BP_FirstPersonCharacter_C|GetHasKey (Variables|Default|GetBP_FirstPersonCharacter))
      (Rendering|Material|SetVectorParameterValue _dynamicmaterial "Colour" "(R=0.000000,G=1.000000,B=0.000000,A=1.000000)" :!class /Script/Engine.MaterialInstanceDynamic)
      ;[0.15 0.15 0.15 0.5] Door Animation
      (bind _alpha (Timeline|Timeline Play)
        (:Update
          (Transformation|SetRelativeRotation (Variables|Default|GetSM_Door) (Math|Rotator|Lerp(Rotator) "0, 0, 0" "0.000000,90.000000,0.000000" _alpha) false false)))
      (else
        (Rendering|Material|SetVectorParameterValue _dynamicmaterial "Colour" "(R=1.000000,G=0.000000,B=0.000000,A=1.000000)" :!class /Script/Engine.MaterialInstanceDynamic)))))

(event OnComponentEndOverlap(DoorCollision)
  (params (OverlappedComponent :type Primitive%20Component%20Object%20Reference) (OtherActor :type Actor%20Object%20Reference) (OtherComp :type Primitive%20Component%20Object%20Reference) (OtherBodyIndex :type Integer))
  (bind _dynamicmaterial (Variables|Default|GetDynamicMaterial))
  ;[0.15 0.15 0.15 0.5] Return Light to Default
  (if (== OtherActor (Variables|Default|GetBP_FirstPersonCharacter))
    (Rendering|Material|SetScalarParameterValue _dynamicmaterial "Colour" 1.0 :!class /Script/Engine.MaterialInstanceDynamic)
    (Rendering|Material|SetVectorParameterValue _dynamicmaterial "Colour" "(R=0.829195,G=1.000000,B=0.364583,A=1.000000)" :!class /Script/Engine.MaterialInstanceDynamic)
    ;[0.15 0.15 0.15 0.5] Door Animation
    (bind _alpha (Timeline|Timeline Reverse)
      (:Update
        (Transformation|SetRelativeRotation (Variables|Default|GetSM_Door) (Math|Rotator|Lerp(Rotator) "0, 0, 0" "0.000000,90.000000,0.000000" _alpha) false false)))))

(event EventBeginPlay
  ;[0.15 0.15 0.15 0.5] Set-up
  (bind _asbp_first_person_character (Utilities|Casting|CastToBP_FirstPersonCharacter (Game|GetPlayerCharacter 0)))
  (Variables|Default|SetBP_FirstPersonCharacter _asbp_first_person_character)
  (bind _returnvalue (Rendering|Material|CreateDynamicMaterialInstance "/Game/MyContent/Materials/MI_Door_Light.MI_Door_Light" "None" "None" :!class /Script/Engine.KismetMaterialLibrary))
  (Variables|Default|SetDynamicMaterial _returnvalue)
  (Rendering|Material|SetMaterial (Variables|Default|GetSM_Light) 0 (Variables|Default|GetDynamicMaterial)))

(fn ConstructionScript)